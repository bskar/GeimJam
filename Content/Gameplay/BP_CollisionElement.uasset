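; BP_CollisionElement is an astronaut actor with health whose defeat hands the aliens the win and whose capsule kills the player character on overlap.
; A looping timer randomly plays hum sounds.
; A bound TakeHit event randomly plays a hit sound and subtracts health, calling AlienWin on the game mode and playing a lose sound at zero.
; Sound plays set a timed AllowSound cooldown flag, which is never checked here.
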(event OnComponentBeginOverlap(Capsule)
  (params (OverlappedComponent :type Primitive%20Component%20Object%20Reference) (OtherActor :type Actor%20Object%20Reference) (OtherComp :type Primitive%20Component%20Object%20Reference) (OtherBodyIndex :type Integer) (bFromSweep :type Boolean) (SweepResult :type Hit%20Result%20Structure%20%28by%20ref%29))
  (if (== OtherActor 0)
    (bind _asthird_person_character (Utilities|Casting|CastToThirdPersonCharacter OtherActor))
    (Default|Kill _asthird_person_character)))

(event Custom|TakeHit_Event
  (if (Math|Random|RandomBool)
    (Audio|PlaySoundatLocation "/Game/Sound/SFX/SC_SpacemanHit.SC_SpacemanHit" (Transformation|GetActorLocation)) ; Play sound randomly
    (Variables|Default|SetAllowSound false)
    (Utilities|Time|SetTimerbyEvent (delegate Custom|AllowSoundAgain) 3.0))
  (bind _output_get (Variables|Default|SetHealth (- (Variables|Default|GetHealth) 2.0)))
  (if (<= _output_get 0.0)
    (bind _asthird_person_game_mode (Utilities|Casting|CastToThirdPersonGameMode (Game|GetGameMode)))
    (Default|AlienWin _asthird_person_game_mode)
    (Audio|PlaySoundatLocation "/Game/Sound/SFX/SC_SpacemanLose.SC_SpacemanLose" (Transformation|GetActorLocation))))

(event Custom|Hum
  (if (Math|Random|RandomBool)
    (Audio|PlaySoundatLocation "/Game/Sound/SFX/SC_HumAstronaut.SC_HumAstronaut" (Transformation|GetActorLocation)) ; Play sound randomly
    (Variables|Default|SetAllowSound false)
    (Utilities|Time|SetTimerbyEvent (delegate Custom|AllowSoundAgain) 3.0)))

(event Custom|AllowSoundAgain
  (Variables|Default|SetAllowSound true))

(event EventBeginPlay
  (EventDispatchers|BindEventtoTakeHit (delegate Custom|TakeHit_Event))
  (Utilities|Time|SetTimerbyEvent (delegate Custom|Hum) 6.0 true))

(fn ConstructionScript)
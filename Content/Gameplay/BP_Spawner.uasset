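; BP_Spawner is a respawn point that revives a player at its location, at a fixed height, with an alien revive sound.
; Collider overlap starts a looping timer that requests a respawn through ThirdPersonGameMode whenever living players are below the player count; ending overlap clears it.
; A CanSpawn flag on the game mode, reset by a delayed timer here, acts as a cooldown shared through the game mode.
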(event OnComponentBeginOverlap(Collider)
  (params (OverlappedComponent :type Primitive%20Component%20Object%20Reference) (OtherActor :type Actor%20Object%20Reference) (OtherComp :type Primitive%20Component%20Object%20Reference) (OtherBodyIndex :type Integer) (bFromSweep :type Boolean) (SweepResult :type Hit%20Result%20Structure%20%28by%20ref%29))
  (bind _returnvalue (Utilities|Time|SetTimerbyEvent (delegate Custom|CheckIfSpawn) 0.3 true))
  (Variables|Default|SetOurTimer _returnvalue))

(event OnComponentEndOverlap(Collider)
  (params (OverlappedComponent :type Primitive%20Component%20Object%20Reference) (OtherActor :type Actor%20Object%20Reference) (OtherComp :type Primitive%20Component%20Object%20Reference) (OtherBodyIndex :type Integer))
  (Utilities|Time|ClearandInvalidateTimerbyHandle (Variables|Default|GetOurTimer)))

(event Custom|ResetSpawn
  (Variables|/Game/Characters/StarterContent/ThirdPersonBP/Blueprints/ThirdPersonGameMode.ThirdPersonGameMode_C|SetCanSpawn (stale Custom|CheckIfSpawn _asthird_person_game_mode) true))

(event Custom|CheckIfSpawn
  (bind _returnvalue (Transformation|GetActorTransform))
  (if (not (== (stale OnComponentBeginOverlap(Collider) OtherActor) "/Game/Characters/StarterContent/ThirdPersonBP/Blueprints/ThirdPersonCharacter.ThirdPersonCharacter_C"))
    (bind _asthird_person_game_mode (Utilities|Casting|CastToThirdPersonGameMode (Game|GetGameMode)))
    (if (< (Variables|/Game/Characters/StarterContent/ThirdPersonBP/Blueprints/ThirdPersonGameMode.ThirdPersonGameMode_C|GetNumberOfLivingPlayers _asthird_person_game_mode) (Variables|/Game/Characters/StarterContent/ThirdPersonBP/Blueprints/ThirdPersonGameMode.ThirdPersonGameMode_C|GetNumberOfPlayers _asthird_person_game_mode))
      (if (Variables|/Game/Characters/StarterContent/ThirdPersonBP/Blueprints/ThirdPersonGameMode.ThirdPersonGameMode_C|GetCanSpawn _asthird_person_game_mode)
        (Variables|/Game/Characters/StarterContent/ThirdPersonBP/Blueprints/ThirdPersonGameMode.ThirdPersonGameMode_C|SetCanSpawn _asthird_person_game_mode false)
        (Utilities|Time|SetTimerbyEvent (delegate Custom|ResetSpawn) 4.0)
        (Default|Respawn _asthird_person_game_mode (Math|Transform|MakeTransform (Math|Vector|MakeVector (.x (.location _returnvalue)) (.y (.location _returnvalue)) 5e+02) (.rotation _returnvalue) (.scale _returnvalue)))
        (Audio|PlaySoundatLocation "/Game/Sound/SFX/SC_ReviveAlien.SC_ReviveAlien" (Transformation|GetActorLocation (stale OnComponentBeginOverlap(Collider) OtherActor)))))))

(event EventBeginPlay)

(fn ConstructionScript)
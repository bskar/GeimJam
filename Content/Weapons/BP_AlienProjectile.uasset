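; Alien weapon projectile that grows after spawning and detects hits on the motion controller pawn.
; A timeline curve scales the root component up from BeginPlay, and the actor destroys itself when the timeline finishes.
; The Cone component's overlap with the pawn prints a debug hit message and destroys the projectile early.
; An ApplyDamage node is present but unwired, so hits deal no damage.
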(event OnComponentBeginOverlap(Cone)
  (params (OverlappedComponent :type Primitive%20Component%20Object%20Reference) (OtherActor :type Actor%20Object%20Reference) (OtherComp :type Primitive%20Component%20Object%20Reference) (OtherBodyIndex :type Integer) (bFromSweep :type Boolean) (SweepResult :type Hit%20Result%20Structure%20%28by%20ref%29))
  (bind _asmotion_controller_pawn (Utilities|Casting|CastToMotionControllerPawn OtherActor))
  (Development|PrintString "HIT!!!!!!!!!!!!!")
  (Actor|DestroyActor))

(event EventBeginPlay
  (bind _growcurve (Timeline|ScaleUp Play)
    (:Update
      (Transformation|SetRelativeScale3D (Variables|Default|GetDefaultSceneRoot) (Math|Vector|MakeVector (Math|Float|Lerp 0.75 4.0 _growcurve) (Math|Float|Lerp 0.75 4.0 _growcurve) (Math|Float|Lerp 0.75 4.0 _growcurve))))
    (:Finished
      (Actor|DestroyActor))))

(event Collision|EventActorBeginOverlap
  (params (OtherActor :type Actor%20Object%20Reference)))

(fn ConstructionScript)